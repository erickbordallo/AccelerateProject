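; AI-controlled player pawn, driven by an AICon_CarBasic controller, that arms itself with a random primary weapon at spawn.
; On BeginPlay it picks either a LaserBlaster or a Flamethrower with equal odds and creates it.
; It then passes the controller a matching weapon range, long for the laser and short for the flamethrower, along with a reference to itself as owner.
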(event EventBeginPlay
  (bind _returnvalue (Pawn|GetController))
  (bind _self self)
  (if (== (Math|Random|RandomIntegerinRange 1 2) 1)
    (Class|AcceleratePlayer|CreatePrimaryWeapon "LaserBlaster")
    (bind _asaicon_car_basic (Utilities|Casting|CastToAICon_CarBasic _returnvalue))
    (Default|SetWeaponRange _asaicon_car_basic 1e+04)
    (Default|SetOwnerRef _asaicon_car_basic _self)
    (else
      (Class|AcceleratePlayer|CreatePrimaryWeapon "Flamethrower")
      (bind _asaicon_car_basic_2 (Utilities|Casting|CastToAICon_CarBasic _returnvalue))
      (Default|SetWeaponRange _asaicon_car_basic_2 2e+03)
      (Default|SetOwnerRef _asaicon_car_basic_2 _self))))

(event Collision|EventActorBeginOverlap
  (params (OtherActor :type Actor%20Object%20Reference)))

(event EventTick
  (params (DeltaSeconds :type Float%20%28single-precision%29)))

(fn ConstructionScript)