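; Base weapon Blueprint that provides firing, shot-delay and overheating logic.
; Fire_Event sets IsFiring and runs a debug-drawn line trace forward from EndOfBarrel, casting the hit to BP_Car with no follow-up yet.
; AutoFire gates FireEvent on CanFire, adds heat and re-arms after a delay unless heat exceeds the maximum.
; ReduceHeatLvl cools the weapon over DeltaTime while not firing, restoring CanFire at or below that limit.
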(event Custom|Fire_Event
  (bind _endofbarrel (Variables|Default|GetEndOfBarrel))
  (bind _returnvalue (Transformation|GetWorldLocation _endofbarrel))
  ;[1 1 1] Fire Event
  (Variables|Default|SetisFiring true)
  (bind _outhit (Collision|LineTraceByChannel _returnvalue (+ _returnvalue (* (Math|Vector|GetForwardVector (Transformation|GetWorldRotation _endofbarrel)) 5e+03)) "TraceTypeQuery1" false 0 "Persistent"))
  (Utilities|Casting|CastToBP_Car (.HitActor (Collision|BreakHitResult _outhit))))

(event Custom|AutoFire
  ;[1 1 1] Auto Fire
  (if (Variables|Default|GetcanFire)
    (CallFunction|FireEvent)
    (CallFunction|AddHeating)
    (Variables|Default|SetcanFire false)
    (if (<= (Variables|Default|GetweaponHeatLvl) (Variables|Default|GetmaxHeatLvl))
      (Utilities|FlowControl|Delay (Variables|Default|GetshotDelay))
      (Variables|Default|SetcanFire true))))

(event Custom|AddHeating
  ;[1 1 1] Add Heating Event
  (Variables|Default|SetweaponHeatLvl (+ (Variables|Default|GetweaponHeatLvl) (Variables|Default|GetheatLvlIncement))))

(event Custom|ReduceHeatLvl
  (params (DeltaTime :type Float%20%28single-precision%29))
  ;[1 1 1] Reduce Heat Event
  (if (not (Variables|Default|GetisFiring))
    (if (> (Variables|Default|GetweaponHeatLvl) 0.0)
      (bind _output_get (Variables|Default|SetweaponHeatLvl (- (Variables|Default|GetweaponHeatLvl) (* DeltaTime (Variables|Default|GetheatLvlReduction)))))
      (if (<= _output_get (Variables|Default|GetmaxHeatLvl))
        (Variables|Default|SetcanFire true)))))

(event Custom|StopFiring
  ;[1 1 1] Stop Fire Event
  (Variables|Default|SetisFiring false))

(fn ConstructionScript)