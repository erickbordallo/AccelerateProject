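; Defensive shield weapon that surrounds an AcceleratePlayer car with a temporary sphere and flags that car as shielded.
; DeployShield sets the active flags and, if ready, plays a sound and runs a timeline that grows the collision sphere and visual together.
; After ShieldDuration it collapses the sphere, clears the flags and becomes ready again.
; While active, Tick accumulates ShieldLiveTime, and GetIsActiveShield exposes the active state.
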(event Custom|DeployShield
  (params (ObjRef :type Object%20Object%20Reference))
  (bind _spherecollision (Variables|Default|GetSphereCollision))
  (bind _spheretexture (Variables|Default|GetSphereTexture))
  ;[1 1 1] Deploy Shield Event
  (bind _asaccelerate_player (Utilities|Casting|CastToAcceleratePlayer ObjRef))
  (bind _output_get (Variables|Default|SetCarRef _asaccelerate_player))
  (Variables|/Script/Accelerate.AcceleratePlayer|SetisShieldActive _output_get true)
  (Variables|Default|SetisActive true)
  (if (Variables|Default|GetisReady)
    (Utilities|FlowControl|Sequence
      (:then_0
        (Audio|PlaySoundatLocation (Variables|Default|GetShieldSound) (Transformation|GetWorldLocation (Variables|Default|GetSphereCollision)) "0, 0, 0" 1.0 1.0 0.0 0 0 0)
        (Components|Activation|Activate _spherecollision true)
        (Components|Activation|Activate _spheretexture true)
        (Variables|Default|SetisReady false))
      (:then_1
        (bind _lerpamount (Timeline|Activate%20Shield PlayFromStart)
          (:Update
            (Components|Sphere|SetSphereRadius _spherecollision (Math|Float|Lerp 0.0 (Variables|Default|GetsphereRadius) _lerpamount) true)
            (Transformation|SetRelativeScale3D _spheretexture (Math|Vector|Lerp(Vector) "0.100000,0.100000,0.100000" (Variables|Default|GetSphereTextureScale) _lerpamount)))
          (:Finished
            (Utilities|FlowControl|Delay (Variables|Default|GetShieldDuration))
            (CallFunction|Init)
            (Variables|Default|SetisReady true)
            (Variables|/Script/Accelerate.AcceleratePlayer|SetisShieldActive (Variables|Default|GetCarRef) false)
            (Variables|Default|SetisActive false)))))))

(event Custom|Init
  (bind _spherecollision (Variables|Default|GetSphereCollision))
  (bind _spheretexture (Variables|Default|GetSphereTexture))
  ;[1 1 1] Initiation
  (Components|Activation|Deactivate _spherecollision)
  (Components|Sphere|SetSphereRadius _spherecollision 0.0 true)
  (Transformation|SetRelativeScale3D _spheretexture "0.100000,0.100000,0.100000")
  (Components|Activation|Deactivate _spheretexture))

(event EventBeginPlay
  ;[1 1 1] Beginplay
  (CallFunction|Init)
  (Variables|Default|SetisReady true))

(event EventTick
  (params (DeltaSeconds :type Float%20%28single-precision%29))
  (if (Variables|Default|GetisActive)
    (Variables|Default|SetshieldLiveTime (+ (Variables|Default|GetshieldLiveTime) (* 17.0 DeltaSeconds)))
    (Utilities|FlowControl|Delay 1.0)))

(fn ConstructionScript)

(fn GetIsActiveShield
  (return (Variables|Default|GetisActive)))