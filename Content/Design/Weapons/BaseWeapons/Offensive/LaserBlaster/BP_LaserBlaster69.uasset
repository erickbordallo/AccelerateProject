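; BP_LaserBlaster69 is a laser blaster weapon that spawns laser projectiles and inherits the speed of the car it rides on.
; Tick derives the current speed from the change in actor location over delta time.
; The fire event spawns BP_LaserProjectile69 at the barrel end, plays a sound at it, and passes in that speed and the weapon's damage.
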(event EventBeginPlay
  ;[1 1 1] Set Position
  (Variables|Default|SetoldPosition (Transformation|GetActorLocation)))

(event EventTick
  (params (DeltaSeconds :type Float%20%28single-precision%29))
  ;[1 1 1] Get car speed and set laser speed
  (Variables|Default|SetSpeed (/ (Math|Vector|VectorLength (- (Transformation|GetActorLocation) (Variables|Default|GetoldPosition))) (Utilities|Time|GetWorldDeltaSeconds)))
  (Variables|Default|SetoldPosition (Transformation|GetActorLocation)))

(event EventLaserBlasterFireEvent
  ;[1 1 1] Spawn Laser when fired, play sound and set damage
  (Physics|GetPhysicsLinearVelocity (Variables|Default|GetGunMesh) "None")
  (bind _returnvalue (Game|SpawnActorfromClass "/Game/Design/Weapons/BaseWeapons/Offensive/LaserBlaster/BP_LaserProJectile69.BP_LaserProjectile69_C" (Transformation|GetWorldTransform (Variables|Default|GetEndOfBarrel)) "Undefined" 0 0))
  (Audio|PlaySoundatLocation (Variables|Default|GetLaserSound) (Transformation|GetWorldLocation (Variables|/Game/Design/Weapons/BaseWeapons/Offensive/LaserBlaster/BP_LaserProJectile69.BP_LaserProjectile69_C|GetLaserMesh _returnvalue)) "0, 0, 0" 1.0 1.0 0.0 0 0 0)
  (Default|AddSpeed _returnvalue (Variables|Default|GetSpeed))
  (Default|SetLaserDamage _returnvalue (Variables|Default|GetmDamage)))

(fn ConstructionScript)