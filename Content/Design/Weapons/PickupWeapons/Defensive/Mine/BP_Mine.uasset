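; Droppable mine weapon that explodes when a car or homing missile overlaps its trigger box.
; The blast fires a radial impulse, effect and sound, then damages and destroys itself only if the other actor casts to AcceleratePlayer.
; Duplicated Mine event and MineSpawn function ground-trace below player 0's car before spawning a mine, adjusting height by tilt.
; Beam and box-stretching helpers are defined but not called here.
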(event OnComponentBeginOverlap(Box)
  (params (OverlappedComponent :type Primitive%20Component%20Object%20Reference) (OtherActor :type Actor%20Object%20Reference) (OtherComp :type Primitive%20Component%20Object%20Reference) (OtherBodyIndex :type Integer) (bFromSweep :type Boolean) (SweepResult :type Hit%20Result%20Structure%20%28by%20ref%29))
  (bind _returnvalue (Utilities|GetClass OtherActor))
  (bind _mesh (Variables|Default|GetMesh))
  (bind _returnvalue_2 (Transformation|GetWorldLocation _mesh))
  ;[1 1 1] Explosion
  (if (or (Utilities|ClassIsChildOf _returnvalue "/Game/Design/Car/BP_Car.BP_Car_C") (Utilities|ClassIsChildOf _returnvalue "/Game/Design/Weapons/PickupWeapons/Offensive/HomingMissile/BP_HomingMissileCPP.BP_HomingMissileCPP_C"))
    (Transformation|SetWorldTransform (Variables|Default|GetExplosion) (Transformation|GetWorldTransform (Variables|Default|GetMesh)) false false)
    (Effects|SpawnEmitteratLocation "/Game/StarterContent/Particles/P_Explosion.P_Explosion" _returnvalue_2)
    (Class|RadialForceComponent|FireImpulse (Variables|Default|GetExplosion))
    (Audio|PlaySoundatLocation (Variables|Explosion|GetExplosionSound) _returnvalue_2 "0, 0, 0" 1.0 1.0 0.0 0 0 0)
    (bind _asaccelerate_player (Utilities|Casting|CastToAcceleratePlayer OtherActor))
    (Class|AcceleratePlayer|ReceiveDamage _asaccelerate_player (Variables|Explosion|GetDamage))
    (Actor|DestroyActor)))

(event EventBeginPlay
  ;[1 1 1] Beam + Trigger
  (Collision|SetCollisionEnabled (Variables|Default|GetBox) "QueryAndPhysics"))

(event Custom|Mine
  (Development|PrintString "Hello")
  (bind _asbp_car (Utilities|Casting|CastToBP_Car (Game|Player|GetPlayerPawn 0)))
  (Variables|Spawn|SetCarRef _asbp_car)
  (Development|PrintString "LineTrace")
  (bind _returnvalue (Collision|LineTraceForObjects (Transformation|GetWorldLocation (Variables|/Script/Engine.Actor|GetRootComponent (Variables|Spawn|GetCarRef))) (+ (Transformation|GetWorldLocation (Variables|/Script/Engine.Actor|GetRootComponent (Variables|Spawn|GetCarRef))) (* (Math|Vector|GetUpVector (Variables|/Script/Engine.Actor|GetRootComponent (Variables|Spawn|GetCarRef))) -75.0)) (Variables|Spawn|GetWorldstatic) false 0 "None"))
  (if _returnvalue
    (if (> (.Z (Math|Vector|BreakVector (Math|Vector|GetUpVector (Variables|/Script/Accelerate.Car|GetMesh (Variables|Spawn|GetCarRef))))) (.Z (Math|Vector|BreakVector (Math|Vector|GetUpVector (Variables|/Game/Design/Car/BP_Car.BP_Car_C|GetMineSpawnLocation (Variables|Spawn|GetCarRef))))))
      (Game|SpawnActorfromClass "BP_Mine_C" (Transformation|GetWorldTransform (Variables|/Game/Design/Car/BP_Car.BP_Car_C|GetMineSpawnLocation (Variables|Spawn|GetCarRef))) "Undefined" 0 0 0)
      (else
        (Game|SpawnActorfromClass "BP_Mine_C" (Math|Conversions|ToTransform(Vector) (Math|Vector|MakeVector (.X (Math|Vector|BreakVector (.Location (Math|Transform|BreakTransform (Transformation|GetWorldTransform (Variables|/Game/Design/Car/BP_Car.BP_Car_C|GetMineSpawnLocation (Variables|Spawn|GetCarRef))))))) (.Y (Math|Vector|BreakVector (.Location (Math|Transform|BreakTransform (Transformation|GetWorldTransform (Variables|/Game/Design/Car/BP_Car.BP_Car_C|GetMineSpawnLocation (Variables|Spawn|GetCarRef))))))) (.Z (Math|Vector|BreakVector (+ (.Location (Math|Transform|BreakTransform (Transformation|GetWorldTransform (Variables|/Script/Accelerate.Car|GetMesh (Variables|Spawn|GetCarRef))))) (* (Math|Vector|GetForwardVector (Variables|/Script/Accelerate.Car|GetMesh (Variables|Spawn|GetCarRef))) -5e+01)))))) "Undefined" 0 0 0)))
    (Audio|PlaySoundatLocation "/Game/Design/Weapons/PickupWeapons/Defensive/Mine/Audio/Blueprints_TextPop03.Blueprints_TextPop03" "0, 0, 0" "0, 0, 0" 1.0 1.0 0.0 0 0 0)))

(fn ConstructionScript)

(fn CreateBeam
  (params (StartLocation :type Vector) (EndLocation :type Vector))
  (bind _returnvalue (Effects|SpawnEmitteratLocation "/Game/StarterContent/Particles/P_Fire.P_Fire" StartLocation))
  (bind _output_get (Variables|Default|SetLaserBeam _returnvalue))
  (Class|ParticleSystemComponent|SetBeamEndPoint _output_get 0 EndLocation))

(fn SkillTriggerBox
  (params (Endlocation :type Vector))
  (bind _lazer_check (Variables|Default|GetLazer%20check))
  (bind _box (Variables|Default|GetBox))
  (bind _returnvalue (Transformation|GetWorldLocation _lazer_check))
  (bind _returnvalue_2 (- Endlocation _returnvalue))
  (bind _returnvalue_3 (Math|Vector|VectorLength _returnvalue_2))
  (bind _returnvalue_4 (/ _returnvalue_3 2.0))
  (Transformation|SetRelativeScale3D (Variables|Default|GetBox) (Math|Vector|MakeVector _returnvalue_4 1.0 1.0))
  (Transformation|SetRelativeLocation _box (+ (Variables|/Script/Engine.SceneComponent|GetRelativeLocation _box) (Math|Vector|MakeVector _returnvalue_4 0.0 0.0)) false false))

(fn MineSpawn
  (Development|PrintString "Hello")
  (bind _asbp_car (Utilities|Casting|CastToBP_Car (Game|Player|GetPlayerPawn 0)))
  (Variables|Spawn|SetCarRef _asbp_car)
  (Development|PrintString "LineTrace")
  (bind _returnvalue (Collision|LineTraceForObjects (Transformation|GetWorldLocation (Variables|/Script/Engine.Actor|GetRootComponent (Variables|Spawn|GetCarRef))) (+ (Transformation|GetWorldLocation (Variables|/Script/Engine.Actor|GetRootComponent (Variables|Spawn|GetCarRef))) (* (Math|Vector|GetUpVector (Variables|/Script/Engine.Actor|GetRootComponent (Variables|Spawn|GetCarRef))) -75.0)) (Variables|Spawn|GetWorldstatic) false 0 "None"))
  (if _returnvalue
    (if (> (.Z (Math|Vector|BreakVector (Math|Vector|GetUpVector (Variables|/Script/Accelerate.Car|GetMesh (Variables|Spawn|GetCarRef))))) (.Z (Math|Vector|BreakVector (Math|Vector|GetUpVector (Variables|/Game/Design/Car/BP_Car.BP_Car_C|GetMineSpawnLocation (Variables|Spawn|GetCarRef))))))
      (Game|SpawnActorfromClass "BP_Mine_C" (Transformation|GetWorldTransform (Variables|/Game/Design/Car/BP_Car.BP_Car_C|GetMineSpawnLocation (Variables|Spawn|GetCarRef))) "Undefined" 0 0 0)
      (else
        (Game|SpawnActorfromClass "BP_Mine_C" (Math|Conversions|ToTransform(Vector) (Math|Vector|MakeVector (.X (Math|Vector|BreakVector (.Location (Math|Transform|BreakTransform (Transformation|GetWorldTransform (Variables|/Game/Design/Car/BP_Car.BP_Car_C|GetMineSpawnLocation (Variables|Spawn|GetCarRef))))))) (.Y (Math|Vector|BreakVector (.Location (Math|Transform|BreakTransform (Transformation|GetWorldTransform (Variables|/Game/Design/Car/BP_Car.BP_Car_C|GetMineSpawnLocation (Variables|Spawn|GetCarRef))))))) (.Z (Math|Vector|BreakVector (+ (.Location (Math|Transform|BreakTransform (Transformation|GetWorldTransform (Variables|/Script/Accelerate.Car|GetMesh (Variables|Spawn|GetCarRef))))) (* (Math|Vector|GetForwardVector (Variables|/Script/Accelerate.Car|GetMesh (Variables|Spawn|GetCarRef))) -5e+01)))))) "Undefined" 0 0 0)))
    (Audio|PlaySoundatLocation "/Game/Design/Weapons/PickupWeapons/Defensive/Mine/Audio/Blueprints_TextPop03.Blueprints_TextPop03" "0, 0, 0" "0, 0, 0" 1.0 1.0 0.0 0 0 0)))

(fn OnRepCarRef)