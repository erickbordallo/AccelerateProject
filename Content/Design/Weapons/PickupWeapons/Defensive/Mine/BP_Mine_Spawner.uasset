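; Mine spawner for the defensive pickup weapon, which deploys a BP_Mine from a car when FireMine is called.
; It compares the up-vector Z of the car's mesh and MineSpawnLocation to choose between that component's transform and a fallback position.
; The fallback keeps the component's X and Y, takes Z from a point offset behind the mesh, and drops rotation.
; A deploy sound plays at the spawner's own location.
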(event Custom|FireMine
  (params (ObjectCar :type BP%20Car%20Object%20Reference))
  (Variables|Default|SetCarRef ObjectCar)
  (if (> (.Z (Math|Vector|BreakVector (Math|Vector|GetUpVector (Variables|/Script/Accelerate.Car|GetMesh (Variables|Default|GetCarRef))))) (.Z (Math|Vector|BreakVector (Math|Vector|GetUpVector (Variables|/Game/Design/Car/BP_Car.BP_Car_C|GetMineSpawnLocation (Variables|Default|GetCarRef))))))
    (Game|SpawnActorfromClass "/Game/Design/Weapons/PickupWeapons/Defensive/Mine/BP_Mine.BP_Mine_C" (Transformation|GetWorldTransform (Variables|/Game/Design/Car/BP_Car.BP_Car_C|GetMineSpawnLocation (Variables|Default|GetCarRef))) "Undefined" 0 0 0)
    (else
      (Game|SpawnActorfromClass "/Game/Design/Weapons/PickupWeapons/Defensive/Mine/BP_Mine.BP_Mine_C" (Math|Conversions|ToTransform(Vector) (Math|Vector|MakeVector (.X (Math|Vector|BreakVector (.Location (Math|Transform|BreakTransform (Transformation|GetWorldTransform (Variables|/Game/Design/Car/BP_Car.BP_Car_C|GetMineSpawnLocation (Variables|Default|GetCarRef))))))) (.Y (Math|Vector|BreakVector (.Location (Math|Transform|BreakTransform (Transformation|GetWorldTransform (Variables|/Game/Design/Car/BP_Car.BP_Car_C|GetMineSpawnLocation (Variables|Default|GetCarRef))))))) (.Z (Math|Vector|BreakVector (+ (.Location (Math|Transform|BreakTransform (Transformation|GetWorldTransform (Variables|/Script/Accelerate.Car|GetMesh (Variables|Default|GetCarRef))))) (* (Math|Vector|GetForwardVector (Variables|/Script/Accelerate.Car|GetMesh (Variables|Default|GetCarRef))) -5e+01)))))) "Undefined" 0 0 0)))
  (Audio|PlaySoundatLocation (Variables|Default|GetMineDeploySound) (Transformation|GetWorldLocation (Variables|Default|GetDefaultSceneRoot)) "0, 0, 0" 1.35 1.0 0.0 0 0 0))

(fn ConstructionScript)